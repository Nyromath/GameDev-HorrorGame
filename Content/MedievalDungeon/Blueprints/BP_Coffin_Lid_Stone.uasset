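; Stone coffin lid that the player slides open with the PickUp input to free a key inside.
; Box overlap with the first-person character opens and closes a gate on that input.
; While still closed, a press plays a stone sound at world origin, then after a short delay a timeline lerps the lid along local Y.
; When finished, it sets Open, blocking further triggers, and makes the referenced BP_Key grabbable.
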(event OnComponentEndOverlap(Box)
  (params (OverlappedComponent :type Primitive%20Component%20Object%20Reference) (OtherActor :type Actor%20Object%20Reference) (OtherComp :type Primitive%20Component%20Object%20Reference) (OtherBodyIndex :type Integer))
  (Utilities|Casting|CastToBP_FirstPersonCharacter OtherActor)
  (Utilities|FlowControl|Gate true) ; enters at Close
)

(event OnComponentBeginOverlap(Box)
  (params (OverlappedComponent :type Primitive%20Component%20Object%20Reference) (OtherActor :type Actor%20Object%20Reference) (OtherComp :type Primitive%20Component%20Object%20Reference) (OtherBodyIndex :type Integer) (bFromSweep :type Boolean) (SweepResult :type Hit%20Result%20Structure%20%28by%20ref%29))
  (Utilities|Casting|CastToBP_FirstPersonCharacter OtherActor)
  (Utilities|FlowControl|Gate true) ; enters at Open
)

(event EventBeginPlay
  (Input|EnableInput (Game|GetPlayerController 0)))

(event Input|ActionEvents|InputActionPickUp
  (params (Key :type Key%20Structure :default "None"))
  (:Pressed
    (Utilities|FlowControl|Gate true
      (:Exit
        (if (not (Variables|Default|GetOpen))
          (Audio|PlaySoundatLocation "/Game/GameAuido/Stone_Coffin.Stone_Coffin" "0, 0, 0" "0, 0, 0" 1.0 1.0 0.0 0 0 0 0)
          (Utilities|FlowControl|Delay 0.2)
          (bind _open (Timeline|Timeline_0 Play)
            (:Update
              (Transformation|SetRelativeLocation (Variables|Default|GetLid) (Math|Vector|MakeVector 0.0 (Math|Float|Lerp (Variables|Default|GetClosePosFloat) (Variables|Default|GetOpenPosFloat) _open) 41.0) false false))
            (:Finished
              (Variables|Default|SetOpen true)
              (bind _asbp_key (Utilities|Casting|CastToBP_Key (Variables|Default|GetKeyInside)))
              (Variables|/Game/MedievalDungeon/Blueprints/BP_Key.BP_Key_C|SetGrabbable _asbp_key true))))))))

(fn ConstructionScript)