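; BP_Pressure_Pad is a one-shot floor trap trigger that sets a linked boulder rolling when the first-person character steps on it.
; Box overlap plays a step sound once and runs the Press timeline, which lowers the Pad mesh slightly; leaving reverses it.
; When the timeline finishes, it calls BeginRoll on the BP_Boulder in InteractsWith, then destroys the pad.
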(event OnComponentBeginOverlap(Box)
  (params (OverlappedComponent :type Primitive%20Component%20Object%20Reference) (OtherActor :type Actor%20Object%20Reference) (OtherComp :type Primitive%20Component%20Object%20Reference) (OtherBodyIndex :type Integer) (bFromSweep :type Boolean) (SweepResult :type Hit%20Result%20Structure%20%28by%20ref%29))
  (Utilities|Casting|CastToBP_FirstPersonCharacter OtherActor)
  (Utilities|FlowControl|DoOnce false
    (:Completed
      (Audio|PlaySound2D "/Game/GameAudio/StepTrap.StepTrap" 1.0 1.0 0.0 0 0)
      (bind _move (Timeline|Press Play)
        (:Update
          (Transformation|SetRelativeLocation (Variables|Default|GetPad) (Math|Vector|MakeVector 0.0 0.0 (Math|Float|Lerp -8e+01 -85.0 _move)) false false))
        (:Finished
          (bind _asbp_boulder (Utilities|Casting|CastToBP_Boulder (Variables|Default|GetInteractsWith)))
          (Default|BeginRoll _asbp_boulder)
          (Actor|DestroyActor))))))

(event OnComponentEndOverlap(Box)
  (params (OverlappedComponent :type Primitive%20Component%20Object%20Reference) (OtherActor :type Actor%20Object%20Reference) (OtherComp :type Primitive%20Component%20Object%20Reference) (OtherBodyIndex :type Integer))
  (Utilities|Casting|CastToBP_FirstPersonCharacter OtherActor)
  (bind _move (Timeline|Press Reverse)
    (:Update
      (Transformation|SetRelativeLocation (Variables|Default|GetPad) (Math|Vector|MakeVector 0.0 0.0 (Math|Float|Lerp -8e+01 -85.0 _move)) false false))
    (:Finished
      (bind _asbp_boulder (Utilities|Casting|CastToBP_Boulder (Variables|Default|GetInteractsWith)))
      (Default|BeginRoll _asbp_boulder)
      (Actor|DestroyActor))))

(fn ConstructionScript)