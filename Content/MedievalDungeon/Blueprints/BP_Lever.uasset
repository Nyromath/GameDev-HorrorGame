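; BP_Lever is a dungeon lever that the first-person player pulls to operate a linked door or portcullis.
; Box overlap opens a gate on the PickUp input, so it only works in range.
; A FlipFlop alternates playing and reversing the LeverPull timeline, which pitches the whole actor between two positions.
; When the timeline finishes, InteractsWith selects the ObjectRef cast and calls OpenDoor or OpenGate.
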(event OnComponentBeginOverlap(Box)
  (params (OverlappedComponent :type Primitive%20Component%20Object%20Reference) (OtherActor :type Actor%20Object%20Reference) (OtherComp :type Primitive%20Component%20Object%20Reference) (OtherBodyIndex :type Integer) (bFromSweep :type Boolean) (SweepResult :type Hit%20Result%20Structure%20%28by%20ref%29))
  ;[1 1 1] Interact
  (Utilities|Casting|CastToBP_FirstPersonCharacter OtherActor)
  (Utilities|FlowControl|Gate true) ; enters at Open
)

(event OnComponentEndOverlap(Box)
  (params (OverlappedComponent :type Primitive%20Component%20Object%20Reference) (OtherActor :type Actor%20Object%20Reference) (OtherComp :type Primitive%20Component%20Object%20Reference) (OtherBodyIndex :type Integer))
  ;[1 1 1] Interact
  (Utilities|Casting|CastToBP_FirstPersonCharacter OtherActor)
  (Utilities|FlowControl|Gate true) ; enters at Close
)

(event EventBeginPlay
  (Input|EnableInput (Game|GetPlayerController 0)))

(event Input|ActionEvents|InputActionPickUp
  (params (Key :type Key%20Structure :default "None"))
  ;[1 1 1] Interact
  (:Pressed
    (Utilities|FlowControl|Gate true
      (:Exit
        (Utilities|FlowControl|FlipFlop
          (:A
            (bind _flipposition (Timeline|LeverPull PlayFromStart)
              (:Update
                (Transformation|SetActorRelativeRotation (Math|Rotator|MakeRotator 0.0 (Math|Float|Lerp (Variables|Default|GetFlipPos1) (Variables|Default|GetFlipPos2) _flipposition) 0.0)))
              (:Finished
                ;[1 1 1] Which Object to Interact With
                (switch string (Variables|Default|GetInteractsWith)
                  (:Door
                    (bind _asbp_crypt_doorway_lever (Utilities|Casting|CastToBP_Crypt_Doorway_Lever (Variables|Default|GetObjectRef)))
                    (Default|OpenDoor _asbp_crypt_doorway_lever))
                  (:Portcullis
                    (bind _asbp_portcullis (Utilities|Casting|CastToBP_Portcullis (Variables|Default|GetObjectRef)))
                    (Default|OpenGate _asbp_portcullis))))))
          (:B
            (Timeline|LeverPull ReverseFromEnd)))))))

(fn ConstructionScript)