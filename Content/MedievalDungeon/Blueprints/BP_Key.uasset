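; BP_Key is a pickup key that changes the lock state of its assigned cell door, presumably unlocking it.
; A box overlap with the first-person character opens and closes a Gate on the PickUp input, so it only works in range.
; When pressed in range, a Grabbable key casts DoorThisFits to BP_Cell_Door, sets its Locked enum, then destroys itself.
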(event OnComponentBeginOverlap(Box)
  (params (OverlappedComponent :type Primitive%20Component%20Object%20Reference) (OtherActor :type Actor%20Object%20Reference) (OtherComp :type Primitive%20Component%20Object%20Reference) (OtherBodyIndex :type Integer) (bFromSweep :type Boolean) (SweepResult :type Hit%20Result%20Structure%20%28by%20ref%29))
  ;[1 1 1] Interact
  (Utilities|Casting|CastToBP_FirstPersonCharacter OtherActor)
  (Utilities|FlowControl|Gate true) ; enters at Open
)

(event OnComponentEndOverlap(Box)
  (params (OverlappedComponent :type Primitive%20Component%20Object%20Reference) (OtherActor :type Actor%20Object%20Reference) (OtherComp :type Primitive%20Component%20Object%20Reference) (OtherBodyIndex :type Integer))
  ;[1 1 1] Interact
  (Utilities|Casting|CastToBP_FirstPersonCharacter OtherActor)
  (Utilities|FlowControl|Gate true) ; enters at Close
)

(event EventBeginPlay
  (Input|EnableInput (Game|GetPlayerController 0)))

(event Input|ActionEvents|InputActionPickUp
  (params (Key :type Key%20Structure :default "None"))
  ;[1 1 1] Interact
  (:Pressed
    (Utilities|FlowControl|Gate true
      (:Exit
        (if (Variables|Default|GetGrabbable)
          (bind _asbp_cell_door (Utilities|Casting|CastToBP_Cell_Door (Variables|Default|GetDoorThisFits)))
          (Variables|/Game/MedievalDungeon/Blueprints/BP_Cell_Door.BP_Cell_Door_C|SetLocked _asbp_cell_door "NewEnumerator1")
          (Actor|DestroyActor))))))

(fn ConstructionScript)