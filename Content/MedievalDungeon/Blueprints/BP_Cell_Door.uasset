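; BP_Cell_Door is an interactive dungeon cell door that the player can unlock and swing open or closed.
; An overlap box gates the PickUp input, so it only responds while the first-person character is inside.
; A lock-state switch prints a locked message, turns Has Key into Unlocked, or flip-flops between opening and closing.
; Separate open and close timelines lerp the mesh yaw between two angle variables.
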(event OnComponentBeginOverlap(Box)
  (params (OverlappedComponent :type Primitive%20Component%20Object%20Reference) (OtherActor :type Actor%20Object%20Reference) (OtherComp :type Primitive%20Component%20Object%20Reference) (OtherBodyIndex :type Integer) (bFromSweep :type Boolean) (SweepResult :type Hit%20Result%20Structure%20%28by%20ref%29))
  ;[1 1 1] Interact
  (Utilities|Casting|CastToBP_FirstPersonCharacter OtherActor)
  (Utilities|FlowControl|Gate true) ; enters at Open
)

(event OnComponentEndOverlap(Box)
  (params (OverlappedComponent :type Primitive%20Component%20Object%20Reference) (OtherActor :type Actor%20Object%20Reference) (OtherComp :type Primitive%20Component%20Object%20Reference) (OtherBodyIndex :type Integer))
  ;[1 1 1] Interact
  (Utilities|Casting|CastToBP_FirstPersonCharacter OtherActor)
  (Utilities|FlowControl|Gate true) ; enters at Close
)

(event EventBeginPlay
  (Input|EnableInput (Game|GetPlayerController 0)))

(event Input|ActionEvents|InputActionPickUp
  (params (Key :type Key%20Structure :default "None"))
  ;[1 1 1] Interact
  (:Pressed
    (Utilities|FlowControl|Gate true
      (:Exit
        (switch Utilities|FlowControl|Switch|SwitchonEnum_DoorUnlockStatus (Variables|Default|GetLocked)
          (:NewEnumerator0
            (Development|PrintString "This Door is Locked."))
          (:NewEnumerator1
            (Development|PrintString "The Door Unlocks!")
            (Variables|Default|SetLocked "NewEnumerator2"))
          (:NewEnumerator2
            (Utilities|FlowControl|FlipFlop
              (:A
                ;[1 1 1] Open Doors
                (bind _dooropen (Timeline|OpenDoor PlayFromStart)
                  (:Update
                    (Transformation|SetRelativeRotation (Variables|Default|GetSM_Cell_Door) (Math|Rotator|MakeRotator 0.0 0.0 (Math|Float|Lerp (Variables|Default|GetDoorClosedFloat) (Variables|Default|GetDoorOpenFloat) _dooropen)) false false))))
              (:B
                ;[1 1 1] Close Doors
                (bind _dooropen_2 (Timeline|CloseDoor ReverseFromEnd)
                  (:Update
                    (Transformation|SetRelativeRotation (Variables|Default|GetSM_Cell_Door) (Math|Rotator|MakeRotator 0.0 0.0 (Math|Float|Lerp (Variables|Default|GetDoorClosedFloat) (Variables|Default|GetDoorOpenFloat) _dooropen_2)) false false)))))))))))

(fn ConstructionScript)