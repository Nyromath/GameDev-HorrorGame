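; BP_Crypt_Doorway is an interactive double door that the player opens and closes with the PickUp input.
; Box overlaps by BP_FirstPersonCharacter open and close a Gate, so input only works within range.
; A FlipFlop alternates opening and closing, playing Door_Opening at world origin both times.
; Separate timelines per leaf and direction lerp each door's yaw, with the closing pair playing in reverse.
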(event OnComponentBeginOverlap(Box)
  (params (OverlappedComponent :type Primitive%20Component%20Object%20Reference) (OtherActor :type Actor%20Object%20Reference) (OtherComp :type Primitive%20Component%20Object%20Reference) (OtherBodyIndex :type Integer) (bFromSweep :type Boolean) (SweepResult :type Hit%20Result%20Structure%20%28by%20ref%29))
  ;[1 1 1] Interact
  (Utilities|Casting|CastToBP_FirstPersonCharacter OtherActor)
  (Utilities|FlowControl|Gate true) ; enters at Open
)

(event OnComponentEndOverlap(Box)
  (params (OverlappedComponent :type Primitive%20Component%20Object%20Reference) (OtherActor :type Actor%20Object%20Reference) (OtherComp :type Primitive%20Component%20Object%20Reference) (OtherBodyIndex :type Integer))
  ;[1 1 1] Interact
  (Utilities|Casting|CastToBP_FirstPersonCharacter OtherActor)
  (Utilities|FlowControl|Gate true) ; enters at Close
)

(event EventBeginPlay
  (Input|EnableInput (Game|GetPlayerController 0)))

(event Input|ActionEvents|InputActionPickUp
  (params (Key :type Key%20Structure))
  ;[1 1 1] Interact
  (:Pressed
    (Utilities|FlowControl|Gate true
      (:Exit
        (Utilities|FlowControl|FlipFlop
          (:A
            (Audio|PlaySoundatLocation "/Game/GameAudio/Door_Opening.Door_Opening" "0, 0, 0" "0, 0, 0" 1.0 1.0 0.0 0 0 0 0)
            ;[1 1 1] Open Doors
            (Utilities|FlowControl|Sequence
              (:then_0
                (bind _dooropen (Timeline|OpenLeftDoor PlayFromStart)
                  (:Update
                    (Transformation|SetRelativeRotation (Variables|Default|GetSM_DoorWay_Large_Door_Left) (Math|Rotator|MakeRotator 0.0 0.0 (Math|Float|Lerp (Variables|Default|GetLeftDoorCloseFloat) (Variables|Default|GetLeftDoorOpenFloat) _dooropen)) false false))))
              (:then_1
                (bind _dooropen_2 (Timeline|OpenRightDoor PlayFromStart)
                  (:Update
                    (Transformation|SetRelativeRotation (Variables|Default|GetSM_DoorWay_Large_Door_Right) (Math|Rotator|MakeRotator 0.0 0.0 (Math|Float|Lerp (Variables|Default|GetRightDoorCloseFloat) (Variables|Default|GetRightDoorOpenFloat) _dooropen_2)) false false))))))
          (:B
            (Audio|PlaySoundatLocation "/Game/GameAudio/Door_Opening.Door_Opening" "0, 0, 0" "0, 0, 0" 1.0 1.0 0.0 0 0 0 0)
            ;[1 1 1] Close Doors
            (Utilities|FlowControl|Sequence
              (:then_0
                (bind _dooropen_3 (Timeline|Timeline_0 ReverseFromEnd)
                  (:Update
                    (Transformation|SetRelativeRotation (Variables|Default|GetSM_DoorWay_Large_Door_Left) (Math|Rotator|MakeRotator 0.0 0.0 (Math|Float|Lerp (Variables|Default|GetLeftDoorCloseFloat) (Variables|Default|GetLeftDoorOpenFloat) _dooropen_3)) false false))))
              (:then_1
                (bind _dooropen_4 (Timeline|Timeline_1 ReverseFromEnd)
                  (:Update
                    (Transformation|SetRelativeRotation (Variables|Default|GetSM_DoorWay_Large_Door_Right) (Math|Rotator|MakeRotator 0.0 0.0 (Math|Float|Lerp (Variables|Default|GetRightDoorCloseFloat) (Variables|Default|GetRightDoorOpenFloat) _dooropen_4)) false false)))))))))))

(fn ConstructionScript)