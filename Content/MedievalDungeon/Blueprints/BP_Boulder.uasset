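; Rolling boulder hazard that damages the first-person character on overlap.
; BeginRoll enables physics simulation on the boulder to set it moving.
; Tick checks the boulder's velocity to spawn or stop an attached rolling sound.
; A hit runs a Delay-timed sequence of bone-break, scream and heartbeat sounds, all played at world origin, and briefly shows the DamageIndicator widget.
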(event Custom|BeginRoll
  ;[1 1 1] Activate Physics
  (Physics|SetSimulatePhysics (Variables|Default|GetBoulder) true))

(event Custom|StartSound
  ;[1 1 1] Boulder making sounds when moving
  (Utilities|IsValid (Variables|Default|GetBoulder%20Sound)
    (:Is%20Not%20Valid
      (bind _returnvalue (Audio|SpawnSoundAttached "/Game/GameAudio/BoulderRollling.BoulderRollling" (Variables|Default|GetBoulder) "None" "0, 0, 0" "0, 0, 0" "KeepRelativeOffset" false 1.0 1.0 0.0 0 0))
      (Variables|Default|SetBoulder%20Sound _returnvalue))))

(event Custom|StopSound
  (bind _boulder_sound (Variables|Default|GetBoulder%20Sound))
  ;[1 1 1] Boulder making sounds when moving
  (Utilities|IsValid _boulder_sound
    (:Is%20Valid
      (Audio|Components|Audio|Stop _boulder_sound))))

(event EventTick
  (params (DeltaSeconds :type Float%20%28single-precision%29))
  ;[1 1 1] Boulder making sounds when moving
  (if (> (Math|Vector|VectorLength (Transformation|GetComponentVelocity (Variables|Default|GetBoulder))) 0.0)
    (CallFunction|StartSound)
    (else
      (CallFunction|StopSound))))

(event Collision|EventActorBeginOverlap
  (params (OtherActor :type Actor%20Object%20Reference))
  ;[1 1 1] Damages Character, Plays damage sounds and displays damage widget
  (bind _asbp_first_person_character (Utilities|Casting|CastToBP_FirstPersonCharacter OtherActor))
  (Game|Damage|ApplyDamage _asbp_first_person_character 5e+01 0 0)
  (Audio|PlaySoundatLocation "/Game/GameAudio/BonesBreak.BonesBreak" "0, 0, 0" "0, 0, 0" 1.0 1.0 0.0 0 0 0 0)
  (Utilities|FlowControl|Delay 0.2)
  (Audio|PlaySoundatLocation "/Game/GameAudio/Man_Scream.Man_Scream" "0, 0, 0" "0, 0, 0" 1.0 1.0 0.0 0 0 0 0)
  (Utilities|FlowControl|Delay 0.2)
  (bind _returnvalue (UserInterface|CreateWidget "/Game/Ui/DamageIndicator.DamageIndicator_C"))
  (UserInterface|Viewport|AddtoViewport _returnvalue 0)
  (Utilities|FlowControl|Delay 0.5)
  (Widget|RemovefromParent _returnvalue)
  (Audio|PlaySoundatLocation "/Game/GameAudio/HeartbeatLong.HeartbeatLong" "0, 0, 0" "0, 0, 0" 1.0 1.0 0.0 0 0 0 0)
  (Utilities|FlowControl|Delay 0.2)
  (Audio|PlaySoundatLocation "/Game/GameAudio/HeartbeatLong.HeartbeatLong" "0, 0, 0" "0, 0, 0" 1.0 1.0 0.0 0 0 0 0)
  (Utilities|FlowControl|Delay 0.2)
  (Audio|PlaySoundatLocation "/Game/GameAudio/HeartbeatLong.HeartbeatLong" "0, 0, 0" "0, 0, 0" 1.0 1.0 0.0 0 0 0 0)
  (Utilities|FlowControl|Delay 0.5)
  (Audio|PlaySoundatLocation "/Game/GameAudio/HeartbeatLong.HeartbeatLong" "0, 0, 0" "0, 0, 0" 1.0 1.0 0.0 0 0 0 0)
  (Utilities|FlowControl|Delay 0.1))

(fn ConstructionScript)